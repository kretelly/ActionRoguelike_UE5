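; An actor that repeatedly spawns magic projectiles and can be switched on and off through interaction.
; A looping timer started on BeginPlay spawns BP_MagicProjectile at the actor's location whenever CanSpawn is true.
; Spawns use zero world rotation, so the actor's own orientation is ignored.
; The Interact event uses a FlipFlop to alternate CanSpawn between true and false, starting with true.
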(event Custom|CustomEvent_0
  (if (Variables|Default|GetCanSpawn)
    (Game|SpawnActorfromClass "/Game/ActionRoguelike/BP_MagicProjectile.BP_MagicProjectile_C" (Math|Transform|MakeTransform (Transformation|GetActorLocation)) "Undefined" 0 0)))

(event EventBeginPlay
  (Utilities|Time|SetTimerbyEvent (delegate Custom|CustomEvent_0) 1.0 true))

(event EventInteract
  (params (InstigatorPawn :type Pawn%20Object%20Reference))
  (Utilities|FlowControl|FlipFlop
    (:A
      (Variables|Default|SetCanSpawn true))
    (:B
      (Variables|Default|SetCanSpawn false))))

(fn ConstructionScript)