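; Sprint action Blueprint for the ActionRoguelike action system that temporarily raises the instigator's movement speed.
; StartAction and StopAction each call the parent C++ implementation, then edit MaxWalkSpeed on the instigator's CharacterMovementComponent.
; Start adds SpeedBonus and stop subtracts it, so the change is relative to the current speed rather than restoring a saved value.
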(event EventStartAction
  (params (Instigator :type Actor%20Object%20Reference))
  (bind _returnvalue (Actor|GetComponentbyClass Instigator "/Script/Engine.CharacterMovementComponent"))
  (|CallParentFunction Instigator) ; Super -> call c++ implementation
  (Variables|/Script/Engine.CharacterMovementComponent|SetMaxWalkSpeed _returnvalue (+ (Variables|/Script/Engine.CharacterMovementComponent|GetMaxWalkSpeed _returnvalue) (Variables|Default|GetSpeedBonus))))

(event EventStopAction
  (params (Instigator :type Actor%20Object%20Reference))
  (bind _returnvalue (Actor|GetComponentbyClass Instigator "/Script/Engine.CharacterMovementComponent"))
  (|CallParentFunction Instigator) ; Super -> call c++ implementation
  (Variables|/Script/Engine.CharacterMovementComponent|SetMaxWalkSpeed _returnvalue (- (Variables|/Script/Engine.CharacterMovementComponent|GetMaxWalkSpeed _returnvalue) (Variables|Default|GetSpeedBonus))))