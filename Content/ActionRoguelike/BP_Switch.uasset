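; BP_Switch is an interactable hand switch that signals a linked spawner actor.
; Each Interact event flips IsDown and snaps the switch handle mesh between two opposite tilts by setting its relative rotation, with no animation.
; Both directions send the same InteractMessage to SpawnerActor, so the spawner receives no switch state through that call.
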(event EventInteract
  (params (InstigatorPawn :type Actor%20Object%20Reference))
  (if (Variables|Default|GetIsDown)
    (Transformation|SetRelativeRotation (Variables|Default|GetSM_Hand_Switch) "30.000000, 0, 0" false false)
    (Variables|Default|SetIsDown false)
    (Class|ARogGameplayInterface|Interact(Message) (Variables|Default|GetSpawnerActor))
    (else
      (Transformation|SetRelativeRotation (Variables|Default|GetSM_Hand_Switch) "-30.000000, 0,0.000000" false false)
      (Variables|Default|SetIsDown true)
      (Class|ARogGameplayInterface|Interact(Message) (Variables|Default|GetSpawnerActor)))))

(fn ConstructionScript)