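; BP_ARogPlayerController is the player controller for the ActionRoguelike game, setting up the local player's UI and a save hotkey.
; When a local controller begins playing, it creates the WBP_Main widget, adds it to the viewport and switches input to game only.
; Pressing L casts the game mode to ARogGameModeBase, writes the save game and prints a confirmation.
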(event EventBeginPlay)

(event EventBlueprintBeginPlayingState
  (if (Pawn|IsLocalController)
    (bind _returnvalue (UserInterface|CreateWidget "/Game/ActionRoguelike/UI/WBP_Main.WBP_Main_C"))
    (UserInterface|Viewport|AddtoViewport _returnvalue 0)
    (Input|SetInputModeGameOnly self)))

(event Input|KeyboardEvents|L
  (params (Key :type Key%20Structure :default "None"))
  (:Pressed
    (bind _asarog_game_mode_base (Utilities|Casting|CastToARogGameModeBase (Game|GetGameMode)))
    (Class|ARogGameModeBase|WriteSaveGame _asarog_game_mode_base)
    (Development|PrintString "WORLD SAVED")))

(fn ConstructionScript)