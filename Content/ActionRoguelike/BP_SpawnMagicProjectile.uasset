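; BP_SpawnMagicProjectile is an interactable turret actor that fires magic projectiles at the player.
; Each interaction toggles spawning on or off through a FlipFlop.
; A looping timer started at BeginPlay spawns a BP_MagicProjectile from the actor's location, aimed at the player pawn, while spawning is enabled.
; Tick also rotates an Arrow component to face the player while active.
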(event Custom|CustomEvent_0
  (if (Variables|Default|GetCanSpawn)
    (Game|SpawnActorfromClass "/Game/ActionRoguelike/BP_MagicProjectile.BP_MagicProjectile_C" (Math|Transform|MakeTransform (Transformation|GetActorLocation) (Math|Rotator|FindLookatRotation (Transformation|GetActorLocation) (Transformation|GetActorLocation (Game|Player|GetPlayerPawn 0)))) "Undefined" 0 0)))

(event EventBeginPlay
  (Utilities|Time|SetTimerbyEvent (delegate Custom|CustomEvent_0) 0.5 true))

(event EventTick
  (params (DeltaSeconds :type Float%20%28single-precision%29))
  (if (Variables|Default|GetCanSpawn)
    (Transformation|SetWorldRotation (Variables|Default|GetArrow) (Math|Rotator|FindLookatRotation (Transformation|GetActorLocation) (Transformation|GetActorLocation (Game|Player|GetPlayerPawn 0))) false false)))

(event EventInteract
  (params (InstigatorPawn :type Actor%20Object%20Reference))
  (Utilities|FlowControl|FlipFlop
    (:A
      (Variables|Default|SetCanSpawn true))
    (:B
      (Variables|Default|SetCanSpawn false))))

(fn ConstructionScript)